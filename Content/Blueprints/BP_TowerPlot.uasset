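; BP_TowerPlot is a clickable plot actor that opens a buying widget, apparently for placing or upgrading towers.
; Cursor hover swaps the floor mesh material as a highlight, and clicks use a FlipFlop to show or hide the widget component.
; BeginPlay caches the BuyingWidget reference and hides it.
; Upgrade handling is unfinished: one event only prints the upgrade type, while TowerStats and SendsUpgrades are empty.
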(event `self.ReceiveBeginPlay`
  (bind _widget (`self.Widget`))
  (bind _asbuying_widget (cast `/Game/Widgets/BuyingWidget` (`WidgetComponent.GetUserWidgetObject` _widget)))
  (set `self.BuyingWidgetREF` _asbuying_widget)
  (`SceneComponent.SetHiddenInGame` _widget true false))

(event `self.StaticMesh.OnBeginCursorOver`
  (params (TouchedComponent :type "PrimitiveComponent Object Reference"))
  ;[1 1 1] Setting green colour of mesh
  (`PrimitiveComponent.SetMaterial` (`self.StaticMesh`) 0 "/Game/Materials/FloorMouseOver.FloorMouseOver"))

(event `self.StaticMesh.OnEndCursorOver`
  (params (TouchedComponent :type "PrimitiveComponent Object Reference"))
  ;[1 1 1] Setting green colour of mesh
  (`PrimitiveComponent.SetMaterial` (`self.StaticMesh`) 0 "/Game/Materials/FloorDefault.FloorDefault"))

(event `TowerStats`)

(event `self.StaticMesh.OnClicked`
  (params (TouchedComponent :type "PrimitiveComponent Object Reference") (ButtonPressed :type "Key Structure"))
  (bind _widget (`self.Widget`))
  (`/Engine/EditorBlueprintResources/StandardMacros.FlipFlop`
    (:`A`
      (`SceneComponent.SetHiddenInGame` _widget false false))
    (:`B`
      (`SceneComponent.SetHiddenInGame` _widget true false))))

(event `SendsUpgrades_1_2`
  (params (UpgradeType :type Integer) (Upgrade :type Integer))
  (`KismetSystemLibrary.PrintString` (`KismetStringLibrary.Conv_IntToString` UpgradeType)))

(fn `SendsUpgrades`
  (params (UpgradeType :type Integer) (Upgrade :type Integer))
  (return))

(fn `UserConstructionScript`)