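; Placement preview actor for towers that follows the mouse cursor over world-static geometry at a fixed height.
; Each tick, a capsule overlap against existing TowerBase actors sets the ghost material red or green and updates the Placable flag.
; PlaceTower deducts the building cost through BP_PlayerCamera, spawns a TowerBase with the ghost's TowerData, initializes it and destroys the ghost, without checking Placable itself.
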(event `self.ReceiveTick`
  (params (DeltaSeconds :type "Float (single-precision)"))
  (bind (_hitresult _returnvalue) (`PlayerController.GetHitResultUnderCursorForObjects` (`GameplayStatics.GetPlayerController` 0) (`|MakeArray` "ObjectTypeQuery1" :!type "EObjectTypeQuery Enum") true))
  (bind (_outactors _returnvalue_2) (`KismetSystemLibrary.CapsuleOverlapActors` (`self.K2_GetActorLocation`) 0.0 0.0 (`|MakeArray` "ObjectTypeQuery1" :!type "EObjectTypeQuery Enum") "/Game/Towers/TowerBase.TowerBase_C"))
  (if _returnvalue_2
    (`PrimitiveComponent.SetMaterial` (`self.Ghost Mesh`) 0 "/Game/Materials/GhostTowerRed.GhostTowerRed")
    (set `self.?Placable` false)
    (else
      (`PrimitiveComponent.SetMaterial` (`self.Ghost Mesh`) 0 "/Game/Materials/GhostTowerGreen.GhostTowerGreen")
      (set `self.?Placable` true)))
  (if _returnvalue
    (`self.K2_SetActorLocation` (`KismetMathLibrary.MakeVector` (.x (`.Location` (`GameplayStatics.BreakHitResult` _hitresult))) (.y (`.Location` (`GameplayStatics.BreakHitResult` _hitresult))) 25.0))
    (if true
      _)))

(event `PlaceTower`
  (bind (_towerdata_name _towerdata_damage _towerdata_range _towerdata_firerate _towerdata_projectilespeed _towerdata_buildingcost) (break `/Game/Towers/TowerStruct` (`self.TowerData`)))
  (bind _asbp_player_camera (cast `/Game/Player/BP_PlayerCamera` (`GameplayStatics.GetPlayerPawn` 0)))
  (`/Game/Player/BP_PlayerCamera.AddingMoney` _asbp_player_camera (* _towerdata_buildingcost -1))
  (bind _returnvalue (`|SpawnActorFromClass` "/Game/Towers/TowerBase.TowerBase_C" (`self.GetTransform`) "AlwaysSpawn" "OverrideRootScale" null (struct) 0 0 0 null))
  (set `/Game/Towers/TowerBase.TowerStruct` (`self.TowerData`) _returnvalue)
  (`self.K2_DestroyActor`)
  (`/Game/Towers/TowerBase.InitializeTower` _returnvalue))

(fn `UserConstructionScript`)