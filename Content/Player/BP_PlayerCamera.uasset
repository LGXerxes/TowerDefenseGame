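; Player camera for a tower defense game that also holds the player's money and handles tower placement and selection.
; BeginPlay creates the tower select and overlay HUDs, then grants starting money through AddingMoney, which refreshes the widgets.
; Left click places a held tower, or traces under the cursor to open, retarget or close the upgrade widget.
; Spring arm handles clamped zoom and right-click-gated yaw; edge-scroll functions exist but are never run.
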(event `self.ReceiveTick`
  (params (DeltaSeconds :type "Float (single-precision)"))
  ;[1 1 1] functino to move left
)

(event `self.ReceiveBeginPlay`
  ;[1 1 1] BEGINPLAY, adding huds
  (`|ExecutionSequence`
    (:`then_0`
      (bind _astower_defense_gamemode (cast `/Game/TowerDefenseGamemode` (`GameplayStatics.GetGameMode`)))
      (set `self.GamemodeREF` _astower_defense_gamemode))
    (:`then_1`
      (bind _returnvalue (`|CreateWidget` "/Game/Player/TowerSelectWidget.TowerSelectWidget_C"))
      (set `/Game/Player/TowerSelectWidget.PlayerReference` self _returnvalue)
      (bind _output_get (set `self.TowerSelectWidget REF` _returnvalue))
      (`UserWidget.AddToViewport` _output_get 0))
    (:`then_2`
      (bind _returnvalue_2 (`|CreateWidget` "/Game/Player/OverlayWidget.OverlayWidget_C"))
      (set `/Game/Player/OverlayWidget.PlayerRef` self _returnvalue_2)
      (bind _output_get_2 (set `self.OverlayWidgetREF` _returnvalue_2))
      (set `/Game/Player/OverlayWidget.GamemodeREF` (`self.GamemodeREF`) _output_get_2)
      (`UserWidget.AddToViewport` _output_get_2 0)
      (`self.AddingMoney` (`self.Starting Money`)))))

(event `AddingMoney`
  (params (MoneyToAdd :type Integer))
  (bind _activetowerupgraderef (`self.ActiveTowerUpgradeREF`))
  ;[1 1 1] AddingMoney
  (set `self.PlayerMoney` (+ MoneyToAdd (`self.PlayerMoney`)))
  (`/Game/Player/TowerSelectWidget.AddedMoney` (`self.TowerSelectWidget REF`))
  (`/Engine/EditorBlueprintResources/StandardMacros.IsValid` _activetowerupgraderef
    (:`Is Valid`
      (`/Game/Player/TowerUpgradeWidget.AddedMoney` _activetowerupgraderef))))

(event `InputAction|LeftClick`
  (params (Key :type "Key Structure"))
  (bind _buildertower_ref (`self.BuilderTower REF`))
  (bind _towerselectwidget_ref (`self.TowerSelectWidget REF`))
  (bind _activetowerupgraderef (`self.ActiveTowerUpgradeREF`))
  (bind _activetowerupgraderef_2 (`self.ActiveTowerUpgradeREF`))
  (:`Pressed`
    ;[1 1 1] Placing Tower
    (`/Engine/EditorBlueprintResources/StandardMacros.IsValid` _buildertower_ref
      (:`Is Valid`
        ;;[1 1 1] Check if tower is placable
        (if (`/Game/Towers/GhostTowerBP.?Placable` _buildertower_ref)
          (`/Game/Towers/GhostTowerBP.PlaceTower` _buildertower_ref)
          (set `/Game/Player/TowerSelectWidget.HasTowerInHand` false _towerselectwidget_ref)
          (`Widget.SetVisibility` (`/Game/Player/TowerSelectWidget.PressQtoCancel` _towerselectwidget_ref) "Hidden")
          (else
            (`KismetSystemLibrary.PrintString` "Something is In the way"))))
      (:`Is Not Valid`
        (bind _astower_base (cast `/Game/Towers/TowerBase` (`.HitActor` (`GameplayStatics.BreakHitResult` (`PlayerController.GetHitResultUnderCursorForObjects` (`GameplayStatics.GetPlayerController` 0) (`|MakeArray` "ObjectTypeQuery5" :!type "EObjectTypeQuery Enum") true))))
          (:`then`
            ;[1 1 1] ?Clicking on tower, update or create upgrade window
            (`/Engine/EditorBlueprintResources/StandardMacros.IsValid` _activetowerupgraderef
              (:`Is Valid`
                (`/Game/Player/TowerUpgradeWidget.HoloSelector` _activetowerupgraderef false)
                (set `/Game/Player/TowerUpgradeWidget.SelectedTower` _astower_base _activetowerupgraderef)
                (`/Game/Player/TowerUpgradeWidget.HoloSelector` _activetowerupgraderef true))
              (:`Is Not Valid`
                (bind _returnvalue (`|CreateWidget` "/Game/Player/TowerUpgradeWidget.TowerUpgradeWidget_C"))
                (`|ExecutionSequence`
                  (:`then_0`
                    (set `/Game/Player/TowerUpgradeWidget.PlayerReference` self _returnvalue))
                  (:`then_1`
                    (set `/Game/Player/TowerUpgradeWidget.SelectedTower` _astower_base _returnvalue)
                    (`UserWidget.AddToViewport` _returnvalue 0)
                    (`/Game/Player/TowerUpgradeWidget.HoloSelector` _returnvalue true))
                  (:`then_2`
                    (set `self.ActiveTowerUpgradeREF` _returnvalue))))))
          (:`CastFailed`
            ;[1 1 1] Not Clicking on tower, remove upgrade widget
            (`/Engine/EditorBlueprintResources/StandardMacros.IsValid` _activetowerupgraderef_2
              (:`Is Valid`
                (`Widget.RemoveFromParent` _activetowerupgraderef_2)
                (`/Game/Player/TowerUpgradeWidget.HoloSelector` _activetowerupgraderef_2 false)
                (set `self.ActiveTowerUpgradeREF` null)))))))))

(event `InputAction|ZoomIn`
  (params (Key :type "Key Structure"))
  ;[1 1 1 1 12] Zoom IN & OUT
  (:`Pressed`
    (`self.Zooming` (* (`self.Zoom Speed`) -1.0))))

(event `InputAction|ZoomOut`
  (params (Key :type "Key Structure"))
  ;[1 1 1 1 12] Zoom IN & OUT
  (:`Pressed`
    (`self.Zooming` (`self.Zoom Speed`))))

(event `InputAxisKey|MouseY`
  (params (AxisValue :type "Float (single-precision)"))
  ;[1 1 1] Rotate Camera
  (`/Engine/EditorBlueprintResources/StandardMacros.Gate` true :!label _label
    (:`Exit`
      (`self.Rotation` (`self.GetInputAxisKeyValue`) (`self.RotationSped`)))))

(event `InputAction|RightClick`
  (params (Key :type "Key Structure"))
  ;[1 1 1] Rotate Camera
  (:`Pressed`
    (goto _label :!via `Open`))
  (:`Released`
    (goto _label :!via `Close`)))

(fn `MoveDown`
  (bind (_returnvalue_x _returnvalue_y) (`KismetMathLibrary.BreakVector2D` (`WidgetLayoutLibrary.GetViewportSize`)))
  (bind _returnvalue (`WidgetLayoutLibrary.GetMousePositionOnViewport`))
  (`SceneComponent.K2_AddRelativeLocation` (`self.Scene`) (* (`KismetMathLibrary.FClamp` (`KismetMathLibrary.NormalizeToRange` (`.Y` (`KismetMathLibrary.BreakVector2D` _returnvalue)) (* _returnvalue_y 0.95) _returnvalue_y)) (0.0 -50.0 0.0)) false false))

(fn `MoveLeft`
  (bind _returnvalue_x (`KismetMathLibrary.BreakVector2D` (`WidgetLayoutLibrary.GetViewportSize`)))
  (bind _zoom_speed (`self.Zoom Speed`))
  (bind _returnvalue (`WidgetLayoutLibrary.GetMousePositionOnViewport`))
  (`SceneComponent.K2_AddRelativeLocation` (`self.Scene`) (* (- 1.0 (`KismetMathLibrary.FClamp` (`KismetMathLibrary.NormalizeToRange` (`KismetMathLibrary.BreakVector2D` _returnvalue) 0.0 (* _returnvalue_x 0.1)))) (`KismetMathLibrary.MakeVector` (+ (* (`KismetMathLibrary.NormalizeToRange` (`SpringArmComponent.TargetArmLength` (`self.SpringArm`)) (`self.Min Zoom`) (`self.Max Zoom`)) _zoom_speed) _zoom_speed))) false false))

(fn `MoveRight`
  (bind _returnvalue_x (`KismetMathLibrary.BreakVector2D` (`WidgetLayoutLibrary.GetViewportSize`)))
  (bind _returnvalue (`WidgetLayoutLibrary.GetMousePositionOnViewport`))
  (`SceneComponent.K2_AddRelativeLocation` (`self.Scene`) (* (`KismetMathLibrary.FClamp` (`KismetMathLibrary.NormalizeToRange` (`KismetMathLibrary.BreakVector2D` _returnvalue) (* _returnvalue_x 0.95) _returnvalue_x)) (-50.0 0.0 0.0)) false false))

(fn `MoveUp`
  (bind (_returnvalue_x _returnvalue_y) (`KismetMathLibrary.BreakVector2D` (`WidgetLayoutLibrary.GetViewportSize`)))
  (bind _returnvalue (`WidgetLayoutLibrary.GetMousePositionOnViewport`))
  (`SceneComponent.K2_AddRelativeLocation` (`self.Scene`) (* (- 1.0 (`KismetMathLibrary.FClamp` (`KismetMathLibrary.NormalizeToRange` (`.Y` (`KismetMathLibrary.BreakVector2D` _returnvalue)) 0.0 (* _returnvalue_y 0.1)))) (0.0 50.0 0.0)) false false))

(fn `Rotation`
  (params (A :type "Float (double-precision)") (B :type "Float (double-precision)"))
  (`SceneComponent.K2_AddWorldRotation` (`self.SpringArm`) (`KismetMathLibrary.MakeRotator` 0.0 0.0 (* A B)) false false))

(fn `UserConstructionScript`)

(fn `Zoom`
  (params (ZoomSpeed :type "Float (double-precision)") (`Min Zoom` :type "Float (double-precision)") (`Max Zoom` :type "Float (double-precision)"))
  (bind _returnvalue (+ ZoomSpeed (`SpringArmComponent.TargetArmLength` (`self.SpringArm`))))
  (if (or (>= _returnvalue `Min Zoom`) (<= _returnvalue `Max Zoom`))
    (set `SpringArmComponent.TargetArmLength` _returnvalue (`self.SpringArm`))
    (return)))

(fn `Zooming`
  (params (A :type "Float (double-precision)"))
  (bind _returnvalue (+ A (`SpringArmComponent.TargetArmLength` (`self.SpringArm`))))
  (if (and (<= (`self.Min Zoom`) _returnvalue) (>= (`self.Max Zoom`) _returnvalue))
    (set `SpringArmComponent.TargetArmLength` _returnvalue (`self.SpringArm`))
    (return)))